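; BP_3DWidget is a demo room video wall that displays an animated UMG widget on a mesh.
; The construction script creates a dynamic material instance of M_WallLogo on the Wall mesh, and Tick feeds the widget component's render target into its WallTexture parameter.
; PLAY starts the BP_Wall widget's wall animation, and a text change event pushes the Text variable into the widget's text block.
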(event Custom|PLAYANIM
  ;[1 1 1] Play animation and set text for Video wall
  (bind _asbp_wall (Utilities|Casting|CastToBP_Wall (UserInterface|GetUserWidgetObject (Variables|Default|GetWidget))))
  (UserInterface|Animation|PlayAnimation _asbp_wall (Variables|/Game/DemoRoom/Blueprints/Advanced/UMG/BP_Wall.BP_Wall_C|GetWallAnimation _asbp_wall) 0.0 1 "Forward" 1.0 false))

(event Custom|OnChanged_Text
  ;[1 1 1] Play animation and set text for Video wall
  (bind _asbp_wall (Utilities|Casting|CastToBP_Wall (UserInterface|GetUserWidgetObject (Variables|Default|GetWidget))))
  (Rendering|Components|TextRender|SetText (Variables|/Game/DemoRoom/Blueprints/Advanced/UMG/BP_Wall.BP_Wall_C|GetTextBlock_134 _asbp_wall) (Utilities|Text|ToText(String) (Variables|TextInput|GetText))))

(event EventTick
  (params (DeltaSeconds :type Float%20%28single-precision%29))
  ;[1 1 1] Set widget render texture target to video wall
  (Rendering|Material|SetTextureParameterValue (Variables|Default|GetMatInst) "WallTexture" (Class|WidgetComponent|GetRenderTarget (Variables|Default|GetWidget))))

(fn ConstructionScript
  (bind _returnvalue (Rendering|Material|CreateDynamicMaterialInstance (Variables|Default|GetWall) 1 "/Game/DemoRoom/Materials/M_WallLogo.M_WallLogo" "None" :!class /Script/Engine.PrimitiveComponent))
  (Variables|Default|SetMatInst _returnvalue))

(fn PLAY
  (CallFunction|PLAYANIM))