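; BP_Screen is a demo room wall screen that shows a swappable video texture and has an animated mesh part.
; LED_Open and LED_Close play a timeline forward or in reverse to slide the StaticMesh along its relative Y axis.
; The construction script gives the Plane a dynamic instance of M_WallVideoPlayer, whose Wall_Video parameter OnChanged_Wall_Texture sets from WallTexture.
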(event Custom|LED_Open
  (bind _staticmesh (Variables|Default|GetStaticMesh))
  (bind _relativelocation (Variables|/Script/Engine.SceneComponent|GetRelativeLocation _staticmesh))
  (bind (_x _y _z) (Math|Vector|BreakVector _relativelocation))
  (bind _newtrack_0 (Timeline|Timeline_0 PlayFromStart)
    (:Update
      (Transformation|SetRelativeLocation _staticmesh (Math|Vector|MakeVector _x (Math|Float|Lerp 0.0 1e+02 _newtrack_0) _z) false false))))

(event Custom|LED_Close
  (bind _staticmesh (Variables|Default|GetStaticMesh))
  (bind _relativelocation (Variables|/Script/Engine.SceneComponent|GetRelativeLocation _staticmesh))
  (bind (_x _y _z) (Math|Vector|BreakVector _relativelocation))
  (bind _newtrack_0 (Timeline|Timeline_0 ReverseFromEnd)
    (:Update
      (Transformation|SetRelativeLocation _staticmesh (Math|Vector|MakeVector _x (Math|Float|Lerp 0.0 1e+02 _newtrack_0) _z) false false))))

(event Custom|OnChanged_Wall_Texture
  (Rendering|Material|SetTextureParameterValue (Variables|Default|GetRef_Mat_Wall) "Wall_Video" (Variables|Default|GetWall_Texture)))

(fn ConstructionScript
  (bind _returnvalue (Rendering|Material|CreateDynamicMaterialInstance (Variables|Default|GetPlane) 0 "/Game/DemoRoom/Textures/Video/M_WallVideoPlayer.M_WallVideoPlayer" "None" :!class /Script/Engine.PrimitiveComponent))
  (Variables|Default|SetRef_Mat_Wall _returnvalue))