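; BP_DynMat is a demo-room screen with a border whose displayed texture can be changed at runtime through dynamic materials.
; The construction script creates dynamic material instances for the screen and border meshes and stores both.
; The OnChanged_Texture event pushes the Texture variable into the screen material's Texture parameter.
; A node that would set the border color is present but never runs.
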(event Custom|OnChanged_Texture
  ;[1 1 1] Chnage Texture Realtime
  (Rendering|Material|SetTextureParameterValue (Variables|Default|GetMatSCRInst) "Texture" (Variables|ScreenTexture|GetTexture)))

(fn ConstructionScript
  ;[1 1 1] Creating dynamic Material Instance for screen and frame
  (bind _returnvalue (Rendering|Material|CreateDynamicMaterialInstance (Variables|Default|GetSCR_SM_Screen) 0 0 "None" :!class /Script/Engine.PrimitiveComponent))
  (Variables|Default|SetMatSCRInst _returnvalue)
  (bind _returnvalue_2 (Rendering|Material|CreateDynamicMaterialInstance (Variables|Default|GetSCR_SM_Border) 0 0 "None" :!class /Script/Engine.PrimitiveComponent))
  (Variables|Default|SetMatBRDRInst _returnvalue_2))