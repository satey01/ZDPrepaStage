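; BP_Physics is a demo-room Blueprint that toggles physics simulation on three static mesh spheres.
; The Physics function sets simulation on all three meshes from the EnablePhysics variable.
; Reset applies DisablePhysics to each mesh, then moves it by a fixed, mostly upward offset from its current world location rather than restoring a stored start position.
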(fn ConstructionScript)

(fn Physics
  ;[1 1 1] Enable physics on spheres
  (Physics|SetSimulatePhysics (Variables|Default|GetStaticMeshComponent1) (Variables|Default|GetEnablePhysics)))

(fn Reset
  ;[1 1 1] Reseting location of static meshes
  (for _array_element (Utilities|Array|MakeArray (Variables|Default|GetStaticMeshComponent1) (Variables|Default|GetStaticMeshComponent2) (Variables|Default|GetStaticMeshComponent0))
    (Physics|SetSimulatePhysics _array_element (Variables|Default|GetDisablePhysics))
    (Transformation|SetWorldLocation _array_element (+ (Transformation|GetWorldLocation _array_element) "0,10.000000,250.000000") false false)))