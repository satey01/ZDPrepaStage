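; Demo Blueprint that spawns a sparks particle emitter at a fixed world location and controls its emission rate and color at runtime.
; On BeginPlay it spawns the emitter and caches a dynamic material instance from it.
; A timeline drives the emitter's Rate parameter over time, while a color-change event writes the Color variable to the material's PartColor parameter.
; A PLAY function wraps a PlayRate call.
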(event Custom|Play_Rate
  ;[1 1 1] starting particles over the period of time
  (bind _rate (Timeline|ParticleRate PlayFromStart)
    (:Update
      (Effects|Components|ParticleSystem|SetFloatParameter (stale EventBeginPlay _returnvalue) "Rate" _rate))))

(event Custom|OnChanged_Color
  ;[1 1 1] Setting an event to change particles color
  (Rendering|Material|SetVectorParameterValue (Variables|Default|GetMatInst) "PartColor" (Variables|ParticlesColor|GetColor) :!class /Script/Engine.MaterialInstanceDynamic))

(event EventBeginPlay
  ;[1 1 1] Spawn an instance of particles at known location
  (bind _returnvalue (Effects|SpawnEmitteratLocation "/Game/DemoRoom/FX/ParticleSystems/Sprite/SP_Sparks.SP_Sparks" "2512.428223,-1397.741211,180.000000"))
  ;[1 1 1] Storing Particle Material reference for later use
  (bind _returnvalue_2 (Rendering|Material|CreateDynamicMaterialInstance _returnvalue 0 0 "None" :!class /Script/Engine.PrimitiveComponent))
  (Variables|Default|SetMatInst _returnvalue_2))

(fn ConstructionScript)

(fn PLAY
  (CallFunction|PlayRate))