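; BP_DemoStand is a configurable display stand for a demo room, showing title, description and example text.
; Its construction script assigns the wall mesh, toggles the wall's visibility and fills the three text render components from string variables.
; It also creates dynamic material instances on the Curve and Wall meshes so each receives its own configurable color.
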(fn ConstructionScript
  (bind _wall (Variables|Default|Getwall))
  (Components|StaticMesh|SetStaticMesh _wall "/Game/DemoRoom/Meshes/Structure/SM_Wall.SM_Wall")
  (Rendering|SetVisibility _wall (Variables|Default|GetNewVar_0) false)
  (Class|ZDTextComponent|SetText (Variables|Default|GetTitle) (Utilities|Text|ToText(String) (Variables|Default|GetTitleText)))
  (Rendering|Components|TextRender|SetText (Variables|Default|GetTextRender) (Utilities|Text|ToText(String) (Variables|Default|GetDescriptionText)))
  (Class|ZDTextComponent|SetText (Variables|Default|GetExample) (Utilities|Text|ToText(String) (Variables|Default|GetExampleText)))
  (bind _returnvalue (Rendering|Material|CreateDynamicMaterialInstance (Variables|Default|GetCurve) 1 0 "None" :!class /Script/Engine.PrimitiveComponent))
  (bind _output_get (Variables|Default|SetNewVar_1 _returnvalue))
  (Rendering|Material|SetVectorParameterValue _output_get "Color" (Variables|Default|GetColor) :!class /Script/Engine.MaterialInstanceDynamic)
  (bind _returnvalue_2 (Rendering|Material|CreateDynamicMaterialInstance (Variables|Default|Getwall) 0 0 "None" :!class /Script/Engine.PrimitiveComponent))
  (bind _output_get_2 (Variables|Default|SetNewVar_2 _returnvalue_2))
  (Rendering|Material|SetVectorParameterValue _output_get_2 "Color" (Variables|Default|GetColor02) :!class /Script/Engine.MaterialInstanceDynamic))